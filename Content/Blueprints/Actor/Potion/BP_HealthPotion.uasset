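; BP_HealthPotion is a pickup actor that applies an instant Gameplay Effect to whatever overlaps its sphere, then destroys itself.
; The overlap event calls the C++ ApplyEffectToTarget with InstantGameplayEffectClass.
; An unconnected Blueprint alternative, ApplyEffectToTarget2, gets the actor's Ability System Component and self-applies a spec of the same effect.
; Destruction follows any overlap, with no check on the actor or the result.
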(event `self.Sphere.OnComponentBeginOverlap`
  (params (OverlappedComponent :type "PrimitiveComponent Object Reference") (OtherActor :type "Actor Object Reference") (OtherComp :type "PrimitiveComponent Object Reference") (OtherBodyIndex :type Integer) (bFromSweep :type Boolean) (SweepResult :type "HitResult Structure (by ref)"))
  ;[0 1 0 0.5] 调用C++方法
  (`self.ApplyEffectToTarget` OtherActor (`self.InstantGameplayEffectClass`))
  (`self.K2_DestroyActor`))

(fn `ApplyEffectToTarget2`
  (params (Actor :type "Actor Object Reference"))
  (locals (LocalASC :type "AbilitySystemComponent Object Reference"))
  (bind _output_get (set `local.LocalASC` (`AbilitySystemBlueprintLibrary.GetAbilitySystemComponent` Actor)))
  (`/Engine/EditorBlueprintResources/StandardMacros.IsValid` _output_get
    (:`Is Valid`
      (`AbilitySystemComponent.BP_ApplyGameplayEffectSpecToSelf` (`local.LocalASC`) (`AbilitySystemComponent.MakeOutgoingSpec` (`local.LocalASC`) (`self.InstantGameplayEffectClass`) 1.0 (`AbilitySystemComponent.MakeEffectContext` (`local.LocalASC`)))))))

(fn `UserConstructionScript`)